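; Race course actor that starts a race from an overlap trigger and ends it at the final checkpoint.
; When the third-person character enters RaceTrigger with no race running, it reveals the starting checkpoint and broadcasts OnRaceStarted.
; It binds to the final checkpoint's reached event to clear the game mode's IsInRace flag, print a finish message and broadcast OnRaceCompleted.
; This graph only reads and clears IsInRace, never setting it.
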(event `self.ReceiveBeginPlay`
  (bind _asbp_race_game_mode (cast `/Game/RaceSystem/BP_RaceGameMode` (`GameplayStatics.GetGameMode`)))
  (set `self.RaceGameMode` _asbp_race_game_mode)
  (add `/Game/RaceSystem/RaceCheckpoints/BP_RaceCheckpoint.OnCheckpointReached` (`self.FinalCheckpoint`) (delegate `ProcessFinishedRace`)))

(event `ProcessFinishedRace`
  (params (Checkpoint :type "/Game/RaceSystem/RaceCheckpoints/BP_RaceCheckpoint Object Reference"))
  (set `/Game/RaceSystem/BP_RaceGameMode.bIsInRace` false (`self.RaceGameMode`))
  (`KismetSystemLibrary.PrintString` "Race Finished")
  (`self.OnRaceCompleted`))

(event `self.RaceTrigger.OnComponentBeginOverlap`
  (params (OverlappedComponent :type "PrimitiveComponent Object Reference") (OtherActor :type "Actor Object Reference") (OtherComp :type "PrimitiveComponent Object Reference") (OtherBodyIndex :type Integer) (bFromSweep :type Boolean) (SweepResult :type "HitResult Structure (by ref)"))
  (if (not (`/Game/RaceSystem/BP_RaceGameMode.bIsInRace` (`self.RaceGameMode`)))
    (cast `/Game/ThirdPerson/Blueprints/BP_ThirdPersonCharacter` OtherActor)
    (`self.SetActorHiddenInGame` (`self.StartingCheckpoint`) false)
    (`self.OnRaceStarted`)))

(fn `UserConstructionScript`)